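; Weapon Blueprint that fires a hitscan shot, knocking hit characters into a physics-driven ragdoll.
; FireWeapon runs a debug-drawn Visibility line trace from BulletSpawn along its forward vector, out to WeaponRange.
; If the hit actor is a Ue4ASP_Character, it enables physics simulation on the mesh and applies a fixed world-space velocity impulse to the hit bone, regardless of shot direction.
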(event `FireWeapon`
  (bind _bulletspawn (`self.BulletSpawn`))
  (bind _returnvalue (`SceneComponent.K2_GetComponentLocation` _bulletspawn))
  (bind _outhit (`KismetSystemLibrary.LineTraceSingle` :`Start` _returnvalue :`End` (+ _returnvalue (* (`SceneComponent.GetForwardVector` _bulletspawn) (`self.WeaponRange`))) :`TraceChannel` "TraceTypeQuery1" :`DrawDebugType` "ForDuration"))
  (`|ExecutionSequence`
    (:`then_0`
      (bind (_bblockinghit _binitialoverlap _time _distance _location _impactpoint _normal _impactnormal _physmat _hitactor _hitcomponent _hitbonename) (`GameplayStatics.BreakHitResult` _outhit))
      (bind _asue_4asp_character (cast `/Game/AnimStarterPack/Ue4ASP_Character` _hitactor))
      (bind _mesh (`Character.Mesh` _asue_4asp_character))
      (`PrimitiveComponent.SetSimulatePhysics` _mesh true)
      (`PrimitiveComponent.AddImpulse` _mesh (1000.0 1000.0 1000.0) _hitbonename true))))

(fn `UserConstructionScript`)