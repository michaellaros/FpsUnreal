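; Enemy character Blueprint that reacts to damage and dies when its health runs out.
; On receiving damage it runs the parent handler, then at zero health plays a death animation and destroys itself after a short delay.
; The construction script creates a dynamic material instance on the mesh and applies the BodyColor variable to tint the body per instance.
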(event `self.OnReceiveDamage`
  (`parent.OnReceiveDamage`)
  (if (<= (`self.Health`) 0)
    (`|ExecutionSequence`
      (:`then_0`
        (`SkeletalMeshComponent.PlayAnimation` (`self.Mesh`) "/Game/AnimStarterPack/Death_2.Death_2" false)
        (`KismetSystemLibrary.Delay` 4.0)
        (`self.K2_DestroyActor`)))))

(fn `UserConstructionScript`
  (bind _returnvalue (`PrimitiveComponent.CreateDynamicMaterialInstance` (`self.Mesh`) 0 null "None"))
  (bind _output_get (set `self.DynamicMaterial` _returnvalue))
  (`MaterialInstanceDynamic.SetVectorParameterValue` _output_get "BodyColor" (`self.BodyColor`)))